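; Cannon projectile for the deadly traps that damages the third-person player character on impact.
; Construction script applies configurable speed, radius-based sphere scale, physics mode and optional material override.
; The first hit only turns on physics simulation, subtracts the CannonDamage data table value from the player's HP, then destroys the projectile after a TimeLeft delay.
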(event `self.Sphere.OnComponentHit`
  (params (HitComponent :type "PrimitiveComponent Object Reference") (OtherActor :type "Actor Object Reference") (OtherComp :type "PrimitiveComponent Object Reference") (NormalImpulse :type "Vector Structure") (Hit :type "HitResult Structure (by ref)"))
  (`/Engine/EditorBlueprintResources/StandardMacros.DoOnce` false
    (:`Completed`
      (`PrimitiveComponent.SetSimulatePhysics` (`self.Sphere`) true)
      (`|ExecutionSequence`
        (:`then_0`
          (bind _aspawn (cast `Pawn` OtherActor))
          (bind _asbp_third_person_character (cast `/Game/ThirdPerson/Blueprints/BP_ThirdPersonCharacter` _aspawn))
          (bind _returnvalue (`|GetDataTableRow` "/Game/NewDataTable.NewDataTable" "CannonDamage")
            (:`then`
              (set `/Game/ThirdPerson/Blueprints/BP_ThirdPersonCharacter.HP` (- (`/Game/ThirdPerson/Blueprints/BP_ThirdPersonCharacter.HP` _asbp_third_person_character) (`.Value_5_B5085E7A48FDAD116677158A82148121` (break `/Game/DataTableStruct` _returnvalue))) _asbp_third_person_character))))
        (:`then_1`
          (`KismetSystemLibrary.Delay` (`self.TimeLeft`))
          (`self.K2_DestroyActor`))))))

(fn `UserConstructionScript`
  (bind _returnvalue (/ (* 2 (`self.ProjectileRadius`)) 100.0))
  (set `ProjectileMovementComponent.InitialSpeed` (`self.ProjectileSpeed`) (`self.ProjectileMovement`))
  (`SceneComponent.SetRelativeScale3D` (`self.Sphere`) (`KismetMathLibrary.MakeVector` _returnvalue _returnvalue _returnvalue))
  (`PrimitiveComponent.SetSimulatePhysics` (`self.Sphere`) (`self.UsePhysics`))
  (`/Engine/EditorBlueprintResources/StandardMacros.IsValid` (`self.ProjectileMaterialOverride`)
    (:`Is Valid`
      (`PrimitiveComponent.SetMaterial` (`self.Sphere`) 0 (`self.ProjectileMaterialOverride`)))))