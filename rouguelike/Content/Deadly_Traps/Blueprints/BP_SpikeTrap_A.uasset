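; Spike trap that raises and retracts its spikes, either on a timed loop or when something overlaps its trigger box.
; Two timelines drive spike height, with state flags blocking reactivation until retraction finishes.
; While rising, the first overlap disables spike collision until the next activation, subtracting data-table damage from BP_ThirdPersonCharacter HP.
; The construction script fits both collision boxes to mesh bounds and applies optional material overrides.
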(event `self.ReceiveBeginPlay`
  ;[1 0 0] Event BeginPlay
  (if (not (`self.ActivateWhenTriggered`))
    (`self.ActivateSpikes`)))

(event `ActivateSpikes`
  ;[1 1 1] Activate spikes behaviour
  (if (`self.CanActivate`)
    (set `self.Activated` true)
    (set `self.CanActivate` false)
    (`PrimitiveComponent.SetCollisionEnabled` (`self.SpikeCollision`) "QueryAndPhysics")
    (bind (_direction _newzlocation) (`Timeline|ActivationTimeline` :!via `PlayFromStart`)
      (:`Update`
        (`SceneComponent.K2_SetRelativeLocation` (`self.SM_Spikes_A`) (`KismetMathLibrary.MakeVector` 0.0 0.0 _newzlocation) false false))
      (:`Finished`
        (set `self.Activated` false)
        (`self.RetractSpikes`)))))

(event `RetractSpikes`
  ;[1 1 1] Retract spikes
  (if (not (`self.Activated`))
    (bind (_direction _newzlocation) (`Timeline|RetractTimeline` :!via `PlayFromStart`)
      (:`Update`
        (`SceneComponent.K2_SetRelativeLocation` (`self.SM_Spikes_A`) (`KismetMathLibrary.MakeVector` 0.0 0.0 _newzlocation) false false))
      (:`Finished`
        (set `self.CanActivate` true)
        (if (not (`self.ActivateWhenTriggered`))
          (`KismetSystemLibrary.Delay` (`self.TimeLoopDelay`))
          (`self.ActivateSpikes`))))))

(event `self.BoxTrigger.OnComponentBeginOverlap`
  (params (OverlappedComponent :type "PrimitiveComponent Object Reference") (OtherActor :type "Actor Object Reference") (OtherComp :type "PrimitiveComponent Object Reference") (OtherBodyIndex :type Integer) (bFromSweep :type Boolean) (SweepResult :type "HitResult Structure (by ref)"))
  (if (and (`self.ActivateWhenTriggered`) (not (`self.Activated`)))
    (`self.ActivateSpikes`)))

(event `self.SpikeCollision.OnComponentBeginOverlap`
  (params (OverlappedComponent :type "PrimitiveComponent Object Reference") (OtherActor :type "Actor Object Reference") (OtherComp :type "PrimitiveComponent Object Reference") (OtherBodyIndex :type Integer) (bFromSweep :type Boolean) (SweepResult :type "HitResult Structure (by ref)"))
  (if (`self.Activated`)
    (`PrimitiveComponent.SetCollisionEnabled` (`self.SpikeCollision`) "NoCollision")
    (bind _asbp_third_person_character (cast `/Game/ThirdPerson/Blueprints/BP_ThirdPersonCharacter` OtherActor))
    (bind _returnvalue (`|GetDataTableRow` "/Game/NewDataTable.NewDataTable" "SpikeTrapDamage")
      (:`then`
        (set `/Game/ThirdPerson/Blueprints/BP_ThirdPersonCharacter.HP` (- (`/Game/ThirdPerson/Blueprints/BP_ThirdPersonCharacter.HP` _asbp_third_person_character) (`.Value_5_B5085E7A48FDAD116677158A82148121` (break `/Game/DataTableStruct` _returnvalue))) _asbp_third_person_character)))))

(fn `UserConstructionScript`
  (bind (_min _max) (`StaticMeshComponent.GetLocalBounds` (`self.SM_Spikes_A`)))
  (bind _returnvalue (/ (+ (* _min -1) _max) 2))
  (`|ExecutionSequence`
    (:`then_0`
      (`BoxComponent.SetBoxExtent` (`self.BoxTrigger`) (* (`.Max` (`StaticMeshComponent.GetLocalBounds` (`self.TrapBase`))) 0.8) true)
      (`BoxComponent.SetBoxExtent` (`self.SpikeCollision`) _returnvalue true)
      (`SceneComponent.K2_SetRelativeLocation` (`self.SpikeCollision`) (`KismetMathLibrary.MakeVector` 0.0 0.0 (.z _returnvalue)) false false))
    (:`then_1`
      (`/Engine/EditorBlueprintResources/StandardMacros.IsValid` (`self.BaseMaterialOverride`)
        (:`Is Valid`
          (`PrimitiveComponent.SetMaterial` (`self.TrapBase`) 0 (`self.BaseMaterialOverride`)))))
    (:`then_2`
      (`/Engine/EditorBlueprintResources/StandardMacros.IsValid` (`self.SpikesMaterialOverride`)
        (:`Is Valid`
          (`PrimitiveComponent.SetMaterial` (`self.SM_Spikes_A`) 0 (`self.SpikesMaterialOverride`)))))))