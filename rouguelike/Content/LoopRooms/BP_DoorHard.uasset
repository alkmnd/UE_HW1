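; BP_DoorHard is a button-lit door that procedurally extends a chain of rooms as the player walks through.
; After a startup delay, the first character overlap blocks every BP_DoorHard, then spawns a random room offset by the door's yaw.
; When the character's Rooms count equals RoomsCount, it spawns BP_RoomFinal instead.
; Timelines slide the door open, close it after a delay, then re-allow only that door for reuse without respawning.
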(event `self.ReceiveBeginPlay`
  (`KismetSystemLibrary.Delay` 13.0)
  (set `self.5sec` true)
  (`self.5secDone`))

(event `5secDone`
  (bind _button (`self.Button`))
  (if (`self.5sec`)
    (if (`self.Allow`)
      (`PrimitiveComponent.SetMaterial` _button 0 "/Game/LoopRooms/M_Accept.M_Accept")
      (else
        (`PrimitiveComponent.SetMaterial` _button 0 "/Game/LoopRooms/M_Blocked.M_Blocked")))))

(event `self.Box.OnComponentBeginOverlap`
  (params (OverlappedComponent :type "PrimitiveComponent Object Reference") (OtherActor :type "Actor Object Reference") (OtherComp :type "PrimitiveComponent Object Reference") (OtherBodyIndex :type Integer) (bFromSweep :type Boolean) (SweepResult :type "HitResult Structure (by ref)"))
  (bind _returnvalue (`SceneComponent.K2_GetComponentToWorld` (`self.Door`)))
  (bind _returnvalue_2 (`KismetMathLibrary.FTrunc` (.yaw (.rotation _returnvalue))))
  (bind _returnvalue_3 (+ (.x (.location _returnvalue)) (`self.XAdditional`)))
  (bind _returnvalue_4 (+ (.y (.location _returnvalue)) (`self.YAdditional`)))
  (if (`self.5sec`)
    (if (`self.Allow`)
      (cast `/Game/ThirdPerson/Blueprints/BP_ThirdPersonCharacter` OtherActor)
      (set `self.Allow` false)
      (if (`self.DudesDeactivated`)
        (bind (_direction _newtrack_1) (`Timeline|DoorOpen` :!via `PlayFromStart` :!label _label)
          (:`Update`
            ;[1 1 1] SelfMove
            (`SceneComponent.K2_SetRelativeLocation` (`self.Door`) (`KismetMathLibrary.VLerp` (0.0 0.0 110.0) (0.0 0.0 340.0) _newtrack_1) false false)
            (`PrimitiveComponent.SetMaterial` (`self.Button`) 0 "/Game/LoopRooms/M_Blocked.M_Blocked")
            (set `self.Activated` true))
          (:`Finished`
            (`KismetSystemLibrary.Delay` 13.0)
            (bind (_direction_2 _newtrack_1_2) (`Timeline|DoorClose` :!via `ReverseFromEnd`)
              (:`Update`
                (`SceneComponent.K2_SetRelativeLocation` (`self.Door`) (`KismetMathLibrary.VLerp` (0.0 0.0 110.0) (0.0 0.0 340.0) _newtrack_1_2) false false))
              (:`Finished`
                (`KismetSystemLibrary.Delay` 13.0)
                (set `self.Allow` true)
                (`PrimitiveComponent.SetMaterial` (`self.Button`) 0 "/Game/LoopRooms/M_Accept.M_Accept")))))
        (else
          ;[1 1 1] Deactevation Of Neighbour Doors
          (bind _outactors (`GameplayStatics.GetAllActorsOfClass` "BP_DoorHard_C"))
          (for _array_element _outactors
            (set `/Game/LoopRooms/BP_DoorHard.Allow` false _array_element)
            (`PrimitiveComponent.SetMaterial` (`/Game/LoopRooms/BP_DoorHard.Button` _array_element) 0 "/Game/LoopRooms/M_Blocked.M_Blocked")
            (set `self.DudesDeactivated` true))
          ;[1 1 1] SpawnAndRotateRoom
          (if (== _returnvalue_2 0)
            (set `self.XAdditional` 0.0)
            (set `self.YAdditional` -600.0)
            (bind _asbp_third_person_character (cast `/Game/ThirdPerson/Blueprints/BP_ThirdPersonCharacter` (`GameplayStatics.GetPlayerCharacter` 0) :!label _label_2))
            (if (== (`/Game/ThirdPerson/Blueprints/BP_ThirdPersonCharacter.Rooms` _asbp_third_person_character) (`/Game/ThirdPerson/Blueprints/BP_ThirdPersonCharacter.RoomsCount` _asbp_third_person_character))
              (`|SpawnActorFromClass` "/Game/LoopRooms/BP_RoomFinal.BP_RoomFinal_C" (`KismetMathLibrary.MakeTransform` (`KismetMathLibrary.MakeVector` _returnvalue_3 _returnvalue_4 -50.0) (`KismetMathLibrary.MakeRotator` 0.0 0.0 (.yaw (.rotation _returnvalue)))) "Undefined" "OverrideRootScale" null null)
              (goto _label :!via `PlayFromStart`)
              (else
                (`|SpawnActorFromClass` (`|GetArrayItem` (`self.Class`) (`KismetMathLibrary.RandomIntegerInRange` 0 3)) (`KismetMathLibrary.MakeTransform` (`KismetMathLibrary.MakeVector` _returnvalue_3 _returnvalue_4 -50.0) (`KismetMathLibrary.MakeRotator` 0.0 0.0 (.yaw (.rotation _returnvalue)))) "Undefined" "OverrideRootScale" null null)
                (goto _label :!via `PlayFromStart`)))
            (elif (== _returnvalue_2 90)
              (set `self.XAdditional` 600.0)
              (set `self.YAdditional` 0.0)
              (goto _label_2)
              (elif (== _returnvalue_2 -90)
                (set `self.XAdditional` -600.0)
                (set `self.YAdditional` 0.0)
                (goto _label_2)
                (elif (== _returnvalue_2 -180)
                  (set `self.XAdditional` 0.0)
                  (set `self.YAdditional` 600.0)
                  (goto _label_2)
                  (elif (== _returnvalue_2 180)
                    (set `self.XAdditional` 0.0)
                    (set `self.YAdditional` 600.0)
                    (goto _label_2)))))))))))

(fn `UserConstructionScript`)